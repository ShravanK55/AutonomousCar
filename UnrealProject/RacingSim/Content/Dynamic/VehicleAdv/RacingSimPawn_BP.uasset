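; RacingSimPawn_BP is a vehicle pawn Blueprint with an autonomous driving mode.
; On Tick, after the parent call, the Autonomous flag gates feeding CalculateSteering and the Throttle variable into VehicleMovement.
; CalculateSteering contains only an unconnected calculation that would map the yaw difference toward the Steering target onto a normalized steering range, so it computes no steering as it stands.
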(event EventBeginPlay)

(event Collision|EventActorBeginOverlap
  (params (OtherActor :type Actor%20Object%20Reference)))

(event EventTick
  (params (DeltaSeconds :type Float%20%28single-precision%29))
  (bind _vehiclemovement (Variables|Default|GetVehicleMovement))
  (|CallParentFunction 0.0)
  (if (Variables|Default|GetAutonomous)
    (Class|WheeledVehicleMovementComponent|SetSteeringInput _vehiclemovement (Utilities|CalculateSteering))
    (Class|WheeledVehicleMovementComponent|SetThrottleInput _vehiclemovement (Variables|Default|GetThrottle))))

(fn ConstructionScript)